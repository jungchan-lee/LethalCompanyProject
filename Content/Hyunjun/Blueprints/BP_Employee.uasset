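; Player employee character with flashlight, shovel, item grabbing and ship or door interaction.
; Input events pass through Server/Client event pairs to flashlight, shovel and grab actions, using BP_LethalPlayerState for shovel and hold state.
; E traces from the head socket along camera view to trigger cargo ship buttons, toggle doors or grab BP_MasterItem components.
; Tick draws that debug trace and moves the PhysicsHandle target ahead of the capsule with camera rotation.
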(event `Key|B`
  (params (Key :type "Key Structure"))
  (:`Released`
    (`self.Dead`)))

(event `self.ReceiveBeginPlay`
  (`self.BindPlayerName`))

(event `self.ReceiveTick`
  (params (DeltaSeconds :type "Float (single-precision)"))
  (bind (_start _end) (`self.CalcLineTracePoint`))
  (`|ExecutionSequence`
    (:`then_0`
      (`KismetSystemLibrary.LineTraceSingleForObjects` :`Start` _start :`End` _end :`ObjectTypes` (`|MakeArray` "ObjectTypeQuery1" "ObjectTypeQuery2" "ObjectTypeQuery3" "ObjectTypeQuery4" "ObjectTypeQuery5" "ObjectTypeQuery6" :!type "EObjectTypeQuery Enum") :`DrawDebugType` "ForOneFrame" :`DrawTime` 0.1))
    (:`then_1`
      (`self.Set Physics Handle Target Location and Rotation`))))

(event `EnhancedInput|/Game/Input/Action/IA_Flashlight`
  (params (ActionValue :type Boolean) (ElapsedSeconds :type "Float (double-precision)") (TriggeredSeconds :type "Float (double-precision)") (InputAction :type "InputAction Object Reference" :default "/Game/Input/Action/IA_Flashlight.IA_Flashlight"))
  (:`Completed`
    (if (`self.CheckIsIngameMode`)
      (`self.ServerFlashlight`))))

(event `ServerFlashlight`
  (`self.ClientFlashlight`))

(event `ClientFlashlight`
  (`self.ToggleFlashlight`))

(event `EnhancedInput|/Game/Input/Action/IA_TurnFlashlight`
  (params (ActionValue :type Boolean) (ElapsedSeconds :type "Float (double-precision)") (TriggeredSeconds :type "Float (double-precision)") (InputAction :type "InputAction Object Reference" :default "/Game/Input/Action/IA_TurnFlashlight.IA_TurnFlashlight"))
  (:`Completed`
    (if (`self.CheckIsIngameMode`)
      (`self.ServerTurnFlashlight`))))

(event `ServerTurnFlashlight`
  (`self.ClientTurnFlashlight`))

(event `ClientTurnFlashlight`
  (`self.ToggleTurnFlashlight`))

(event `EnhancedInput|/Game/Input/Action/IA_Shovel`
  (params (ActionValue :type Boolean) (ElapsedSeconds :type "Float (double-precision)") (TriggeredSeconds :type "Float (double-precision)") (InputAction :type "InputAction Object Reference" :default "/Game/Input/Action/IA_Shovel.IA_Shovel"))
  (bind _is_ingame (`self.CheckIsIngameMode`))
  (:`Completed`
    (`KismetSystemLibrary.PrintString` "Completed")
    (if _is_ingame
      _
      (else
        _))
    (`KismetSystemLibrary.PrintString` (`KismetStringLibrary.Conv_BoolToString` _is_ingame))
    (`self.ServerShovel`)))

(event `ServerShovel`
  (`self.ClientShovel`))

(event `ClientShovel`
  (`self.ToggleShovel`))

(event `EnhancedInput|/Game/Input/Action/IA_ShovelAttack`
  (params (ActionValue :type Boolean) (ElapsedSeconds :type "Float (double-precision)") (TriggeredSeconds :type "Float (double-precision)") (InputAction :type "InputAction Object Reference" :default "/Game/Input/Action/IA_ShovelAttack.IA_ShovelAttack"))
  (:`Completed`
    (if (`self.CheckIsIngameMode`)
      (bind _asbp_lethal_player_state (cast `/Game/Hyunjun/Blueprints/Ingame/BP_LethalPlayerState` (`self.PlayerState`)))
      (if (`LethalPlayerState.IsShovel` _asbp_lethal_player_state)
        (`self.ServerShovelAttack`)))))

(event `ServerShovelAttack`
  (`self.ClientShovelAttack`))

(event `ClientShovelAttack`
  (`self.PlayShovelAttack`))

(event `Key|Z`
  (params (Key :type "Key Structure"))
  (:`Pressed`
    (bind _returnvalue (`GameplayStatics.GetActorOfClass` "/DungeonPlugin3/missiontominerva/Actors/KB3D_MTM_VehicleCargoShip_A.KB3D_MTM_VehicleCargoShip_A_C"))
    (bind _askb3d_mtm_vehicle_cargo_ship_a (cast `/DungeonPlugin3/missiontominerva/Actors/KB3D_MTM_VehicleCargoShip_A` _returnvalue))
    (`/DungeonPlugin3/missiontominerva/Actors/KB3D_MTM_VehicleCargoShip_A.LabberAction` _askb3d_mtm_vehicle_cargo_ship_a)))

(event `Key|E`
  (params (Key :type "Key Structure"))
  (bind (_start _end) (`self.CalcLineTracePoint`))
  (:`Pressed`
    (bind _outhit (`KismetSystemLibrary.LineTraceSingleForObjects` :`Start` _start :`End` _end :`ObjectTypes` (`|MakeArray` "ObjectTypeQuery1" "ObjectTypeQuery2" "ObjectTypeQuery3" "ObjectTypeQuery4" "ObjectTypeQuery5" "ObjectTypeQuery6" :!type "EObjectTypeQuery Enum") :`DrawTime` 0.1))
    (`|ExecutionSequence`
      (:`then_0`
        (bind (_bblockinghit _binitialoverlap _time _distance _location _impactpoint _normal _impactnormal _physmat _hitactor _hitcomponent) (`GameplayStatics.BreakHitResult` _outhit))
        (bind _askb3d_mtm_vehicle_cargo_ship_a (cast `/DungeonPlugin3/missiontominerva/Actors/KB3D_MTM_VehicleCargoShip_A` _hitactor))
        (if (== _hitcomponent (`/DungeonPlugin3/missiontominerva/Actors/KB3D_MTM_VehicleCargoShip_A.OpenCloseButton` _askb3d_mtm_vehicle_cargo_ship_a))
          (`/DungeonPlugin3/missiontominerva/Actors/KB3D_MTM_VehicleCargoShip_A.Event_OpenCloseDoor` _askb3d_mtm_vehicle_cargo_ship_a)
          (elif (== _hitcomponent (`/DungeonPlugin3/missiontominerva/Actors/KB3D_MTM_VehicleCargoShip_A.CraneLightButton` _askb3d_mtm_vehicle_cargo_ship_a))
            (`/DungeonPlugin3/missiontominerva/Actors/KB3D_MTM_VehicleCargoShip_A.Event_TurnCraneLight` _askb3d_mtm_vehicle_cargo_ship_a)
            (elif (== _hitcomponent (`/DungeonPlugin3/missiontominerva/Actors/KB3D_MTM_VehicleCargoShip_A.CeilingLightButton` _askb3d_mtm_vehicle_cargo_ship_a))
              (`/DungeonPlugin3/missiontominerva/Actors/KB3D_MTM_VehicleCargoShip_A.Event_TurnCeilingLight` _askb3d_mtm_vehicle_cargo_ship_a)
              (elif (== _hitcomponent (`/DungeonPlugin3/missiontominerva/Actors/KB3D_MTM_VehicleCargoShip_A.CatwalkLightButton` _askb3d_mtm_vehicle_cargo_ship_a))
                (`/DungeonPlugin3/missiontominerva/Actors/KB3D_MTM_VehicleCargoShip_A.Event_TurnCatWalkLight` _askb3d_mtm_vehicle_cargo_ship_a)
                (elif (== _hitcomponent (`/DungeonPlugin3/missiontominerva/Actors/KB3D_MTM_VehicleCargoShip_A.BlastOffLabberEvent` _askb3d_mtm_vehicle_cargo_ship_a))
                  (`/DungeonPlugin3/missiontominerva/Actors/KB3D_MTM_VehicleCargoShip_A.LabberAction` _askb3d_mtm_vehicle_cargo_ship_a)))))))
      (:`then_1`
        (bind _asbp_door (cast `/DungeonPlugin3/Room/BP_Door` _hitactor))
        ;[1 1 1] 코멘트
        (if (== _hitcomponent (`/DungeonPlugin3/Room/BP_Door.Door` _asbp_door))
          (`/DungeonPlugin3/Room/BP_Door.ToggleDoor` _asbp_door)
          (else
            ;[1 1 1] 코멘트
            (if (== _hitcomponent (`/DungeonPlugin3/Room/BP_Door.SM_DoorScreen` _asbp_door))
              (`/DungeonPlugin3/Room/BP_Door.ToggleDoor` _asbp_door)))))
      (:`then_2`
        (`self.ServerGrab` _impactpoint _hitcomponent _hitactor)))))

(event `ServerGrab`
  (params (`Impact Point` :type "Vector Structure") (`Hit Component` :type "PrimitiveComponent Object Reference") (`Hit Actor` :type "Actor Object Reference"))
  (`self.ClientGrab` `Impact Point` `Hit Component` `Hit Actor`))

(event `ClientGrab`
  (params (`Impact Point` :type "Vector Structure") (`Hit Component` :type "PrimitiveComponent Object Reference") (`Hit Actor` :type "Actor Object Reference"))
  (`self.GrabItem` `Impact Point` `Hit Component` `Hit Actor`))

(fn `BindPlayerName`)

(fn `CalcLineTracePoint`
  (returns (Start :type "Vector Structure") (End :type "Vector Structure"))
  (bind _camera (`self.Camera`))
  (return (`SceneComponent.GetSocketLocation` (`self.Mesh`) "head") (+ (0.0 0.0 0.0) (+ (`SceneComponent.K2_GetComponentLocation` _camera) (* (`SceneComponent.GetForwardVector` _camera) 1000.0)))))

(fn `CheckIsIngameMode`
  (returns (`Is Ingame` :type Boolean))
  (cast `/Game/Hyunjun/Blueprints/Ingame/BP_LethalPlayerState` (`self.PlayerState`))
  (return true))

(fn `GrabItem`
  (params (`Impact Point` :type "Vector Structure") (`Hit Component` :type "PrimitiveComponent Object Reference") (`Hit Actor` :type "Actor Object Reference"))
  (locals (IsHold :type Boolean :default false))
  (bind _asbp_lethal_player_state (cast `/Game/Hyunjun/Blueprints/Ingame/BP_LethalPlayerState` (`self.PlayerState`)))
  (if (`LethalPlayerState.IsHold` _asbp_lethal_player_state)
    (bind _asbp_lethal_player_state_2 (cast `/Game/Hyunjun/Blueprints/Ingame/BP_LethalPlayerState` (`self.PlayerState`)))
    (set `LethalPlayerState.IsHold` false _asbp_lethal_player_state_2)
    (`PhysicsHandleComponent.ReleaseComponent` (`self.PhysicsHandle`))
    (else
      (cast `/DungeonPlugin3/Room/Prop/BP_MasterItem` `Hit Actor`)
      (bind _asbp_lethal_player_state_3 (cast `/Game/Hyunjun/Blueprints/Ingame/BP_LethalPlayerState` (`self.PlayerState`)))
      (set `LethalPlayerState.IsHold` true _asbp_lethal_player_state_3)
      (`PhysicsHandleComponent.GrabComponentAtLocationWithRotation` :`self` (`self.PhysicsHandle`) :`Component` `Hit Component` :`Location` `Impact Point`))))

(fn `Set Physics Handle Target Location and Rotation`
  (bind _capsulecomponent (`self.CapsuleComponent`))
  (bind (_returnvalue_roll _returnvalue_pitch _returnvalue_yaw) (`KismetMathLibrary.BreakRotator` (`SceneComponent.K2_GetComponentRotation` (`self.Camera`))))
  (`PhysicsHandleComponent.SetTargetLocationAndRotation` (`self.PhysicsHandle`) (`KismetMathLibrary.MakeVector` (.x (+ (`SceneComponent.K2_GetComponentLocation` _capsulecomponent) (* (`SceneComponent.GetForwardVector` _capsulecomponent) 150.0))) (.y (+ (`SceneComponent.K2_GetComponentLocation` _capsulecomponent) (* (`SceneComponent.GetForwardVector` _capsulecomponent) 150.0))) (+ (.z (+ (`SceneComponent.K2_GetComponentLocation` _capsulecomponent) (* (`SceneComponent.GetForwardVector` _capsulecomponent) 150.0))) 50.0)) (`KismetMathLibrary.MakeRotator` _returnvalue_roll _returnvalue_pitch _returnvalue_yaw)))

(fn `UserConstructionScript`)